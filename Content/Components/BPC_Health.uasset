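; BPC_Health is a health component that tracks an actor's current health and whether it is dead.
; ChangeValue adds a signed amount to CurrentHealth while the owner is alive.
; When health drops to zero or below, it fires the HasDied dispatcher and sets Isdead, which blocks further changes.
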(event `self.ReceiveBeginPlay`)

(fn `ChangeValue`
  (params (Amount :type "Float (double-precision)"))
  (if (not (`self.isdead?`))
    (set `self.CurrentHealth` (+ (`self.CurrentHealth`) Amount))
    (if (<= (`self.CurrentHealth`) 0.0)
      (`self.HasDied`)
      (set `self.isdead?` true))))