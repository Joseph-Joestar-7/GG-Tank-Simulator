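; Destructible vehicle actor (bus by default naming) that rides a spline and can be destroyed by damage.
; On BeginPlay it starts moving: a timeline, rate-scaled by the completion time, sets location and rotation along the assigned spline.
; Damage feeds the health component and a widget health bar that turns toward the camera each Tick.
; Death stops movement, plays explosion sound and fire, hides the bar and swaps to the damaged mesh.
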(event `StopMoving`
  (`TimelineComponent.Stop` (`self.T_move`)))

(event `self.ReceiveBeginPlay`
  (`self.SetActorHiddenInGame` true)
  (`self.move object` 0.0 (`self.spline to follow`))
  (bind _aswbp_vehicle_hb (cast `/Game/UI/WBP_VehicleHB` (`WidgetComponent.GetWidget` (`self.Widget`))))
  (set `self.Hbar` _aswbp_vehicle_hb))

(event `self.BPC_Health.HasDied`
  (`self.StopMoving`)
  (`GameplayStatics.PlaySoundAtLocation` "/Game/Audio/GL_ExplodeIncendiary.GL_ExplodeIncendiary" (`self.K2_GetActorLocation`) (struct) 1.0 1.0 0.0 null null null null)
  (`ActorComponent.Activate` (`self.P_Fire_Big`) true)
  (`SceneComponent.SetVisibility` (`self.damage_bus`) true false)
  (`SceneComponent.SetVisibility` (`self.SM_BUS_01a`) false false)
  (`SceneComponent.SetVisibility` (`self.Widget`) false false))

(event `move object`
  (params (Duration :type "Float (single-precision)") (`spline to follow` :type "/Game/Actors/BP_splinePath Object Reference"))
  (bind _spline (`/Game/Actors/BP_splinePath.Spline` (`self.spline to follow`)))
  (`self.SetActorHiddenInGame` false)
  (set `self.spline to follow` `spline to follow`)
  (`KismetSystemLibrary.Delay` Duration)
  (`TimelineComponent.SetPlayRate` (`self.T_move`) (/ 1.0 (`self.time to complet`)))
  (bind (_direction _move_track) (`Timeline|T_move`)
    (:`Update`
      (if true
        (bind _returnvalue (`KismetMathLibrary.Lerp` 0.0 (`SplineComponent.GetSplineLength` _spline) _move_track))
        (`self.K2_SetActorLocation` (`SplineComponent.GetLocationAtDistanceAlongSpline` _spline _returnvalue "World"))
        (`self.K2_SetActorRotation` (`SplineComponent.GetRotationAtDistanceAlongSpline` _spline _returnvalue "World"))))
    (:`Finished`
      (`TimelineComponent.Stop` (`self.T_move`)))))

(event `self.ReceiveAnyDamage`
  (params (Damage :type "Float (single-precision)") (DamageType :type "DamageType Object Reference") (InstigatedBy :type "Controller Object Reference") (DamageCauser :type "Actor Object Reference"))
  (bind _bpc_health (`self.BPC_Health`))
  (`/Game/Components/BPC_Health.ChangeValue` _bpc_health (* Damage -1.0))
  (`/Game/UI/WBP_VehicleHB.Set Health Bar` (`self.Hbar`) (/ (`/Game/Components/BPC_Health.CurrentHealth` _bpc_health) (`/Game/Components/BPC_Health.MaxHealth` _bpc_health))))

(event `self.ReceiveTick`
  (params (DeltaSeconds :type "Float (single-precision)"))
  (bind _widget (`self.Widget`))
  (`SceneComponent.K2_SetWorldRotation` _widget (`KismetMathLibrary.FindLookAtRotation` (`SceneComponent.K2_GetComponentLocation` _widget) (`SceneComponent.K2_GetComponentLocation` (`PlayerCameraManager.TransformComponent` (`GameplayStatics.GetPlayerCameraManager` 0)))) false false))

(fn `UserConstructionScript`
  (`StaticMeshComponent.SetStaticMesh` (`self.SM_BUS_01a`) (`self.object mesh`)))