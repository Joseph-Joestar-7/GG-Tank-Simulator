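; Stationary turret actor that auto-targets and damages actors carrying a BP_TankWeapon component inside its detection sphere.
; Overlap starts looping timers: Track smoothly rotates the mesh toward the target, while Shoot line-traces from the arrow to apply damage.
; Timers clear when the target leaves or is destroyed.
; Damage feeds the health component and camera-facing health bar; death triggers an explosion and hides turret and bar.
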(event `self.ReceiveTick`
  (params (DeltaSeconds :type "Float (single-precision)"))
  (bind _widget (`self.Widget`))
  (`SceneComponent.K2_SetWorldRotation` _widget (`KismetMathLibrary.FindLookAtRotation` (`SceneComponent.K2_GetComponentLocation` _widget) (`SceneComponent.K2_GetComponentLocation` (`PlayerCameraManager.TransformComponent` (`GameplayStatics.GetPlayerCameraManager` 0)))) false false))

(event `self.ReceiveBeginPlay`
  (bind _aswbp_vehicle_hb (cast `/Game/UI/WBP_VehicleHB` (`WidgetComponent.GetWidget` (`self.Widget`))))
  (set `self.Hbar` _aswbp_vehicle_hb))

(event `self.DetectionSphere.OnComponentBeginOverlap`
  (params (OverlappedComponent :type "PrimitiveComponent Object Reference") (OtherActor :type "Actor Object Reference") (OtherComp :type "PrimitiveComponent Object Reference") (OtherBodyIndex :type Integer) (bFromSweep :type Boolean) (SweepResult :type "HitResult Structure (by ref)"))
  (if (not (`/Game/Components/BPC_Health.isdead?` (`self.BPC_Health`)))
    (`/Engine/EditorBlueprintResources/StandardMacros.IsValid` (`self.GetComponentByClass` OtherActor "/Game/YI_TankCollection/Blueprint/Master/Components/BP_TankWeapon.BP_TankWeapon_C")
      (:`Is Valid`
        (set `self.CurrentTarget` OtherActor)
        (bind _returnvalue (`KismetSystemLibrary.K2_SetTimerDelegate` (delegate `Track`) 0.1 true))
        (set `self.TrackingTimer` _returnvalue)
        (bind _returnvalue_2 (`KismetSystemLibrary.K2_SetTimerDelegate` (delegate `Shoot`) 1.0 true))
        (set `self.DamageTimer` _returnvalue_2)
        (add `self.OnDestroyed` (`self.CurrentTarget`) (delegate `OnDestroyed_Event`))))))

(event `OnDestroyed_Event` :!signature `self.OnDestroyed`
  (params (DestroyedActor :type "Actor Object Reference"))
  (`self.InvalidateTimers`)
  (set `self.CurrentTarget` null))

(event `Track`
  (bind _currenttarget (`self.CurrentTarget`)
    (:`then`
      (`SceneComponent.K2_SetWorldRotation` (`self.SM_Turret`) (`KismetMathLibrary.RInterpTo` (`SceneComponent.K2_GetComponentRotation` (`self.SM_Turret`)) (`KismetMathLibrary.FindLookAtRotation` (`SceneComponent.K2_GetComponentLocation` (`self.Arrow`)) (`self.K2_GetActorLocation` _currenttarget)) (`GameplayStatics.GetWorldDeltaSeconds`) 10.0) false false))
    (:`else`)))

(event `Shoot`
  (bind _arrow (`self.Arrow`))
  (bind _currenttarget (`self.CurrentTarget`))
  (bind _returnvalue (`SceneComponent.K2_GetComponentLocation` _arrow))
  (`|ExecutionSequence`
    (:`then_0`
      (bind (_outhits _returnvalue_2) (`KismetSystemLibrary.LineTraceMulti` _returnvalue (+ _returnvalue (* (`SceneComponent.GetForwardVector` _arrow) 20000.0)) "TraceTypeQuery1"))
      (if _returnvalue_2
        (for _array_element _outhits
          (if (== (`.HitActor` (`GameplayStatics.BreakHitResult` _array_element)) _currenttarget)
            (`GameplayStatics.ApplyDamage` _currenttarget (`self.Base Damage`) null self)))))
    (:`then_1`
      (`GameplayStatics.SpawnEmitterAtLocation` "/Game/YI_TankCollection/Particles/Master/P_Impact_Metal.P_Impact_Metal" _returnvalue (struct :`Pitch` -90.0)))))

(event `self.DetectionSphere.OnComponentEndOverlap`
  (params (OverlappedComponent :type "PrimitiveComponent Object Reference") (OtherActor :type "Actor Object Reference") (OtherComp :type "PrimitiveComponent Object Reference") (OtherBodyIndex :type Integer))
  (if (== OtherActor (`self.CurrentTarget`))
    (set `self.CurrentTarget` null)
    (`self.InvalidateTimers`)))

(event `InvalidateTimers`
  (`KismetSystemLibrary.K2_ClearAndInvalidateTimerHandle` (`self.TrackingTimer`))
  (`KismetSystemLibrary.K2_ClearAndInvalidateTimerHandle` (`self.DamageTimer`)))

(event `self.ReceiveAnyDamage`
  (params (Damage :type "Float (single-precision)") (DamageType :type "DamageType Object Reference") (InstigatedBy :type "Controller Object Reference") (DamageCauser :type "Actor Object Reference"))
  (bind _bpc_health (`self.BPC_Health`))
  (`/Game/Components/BPC_Health.ChangeValue` (`self.BPC_Health`) (* Damage -1.0))
  (`/Game/UI/WBP_VehicleHB.Set Health Bar` (`self.Hbar`) (/ (`/Game/Components/BPC_Health.CurrentHealth` _bpc_health) (`/Game/Components/BPC_Health.MaxHealth` _bpc_health))))

(event `self.BPC_Health.HasDied`
  (`self.InvalidateTimers`)
  (`ActorComponent.Activate` (`self.P_Explosion_Big_A`) true)
  (`SceneComponent.SetVisibility` (`self.Widget`) false false)
  (`SceneComponent.SetVisibility` (`self.SM_Turret`) false false))

(fn `UserConstructionScript`)