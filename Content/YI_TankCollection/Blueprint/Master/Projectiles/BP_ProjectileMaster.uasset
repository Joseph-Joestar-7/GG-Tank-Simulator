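; BP_ProjectileMaster is the tank collection's projectile, configurable as missile or bullet, with construction-set speed and gravity.
; On hitting anything but its owner, it applies damage and radial impulse on the server and sphere-traces for the physical material.
; Surface type drives impact effects and decals, with metal skipping decals and reporting damage to the owning tank controller's UI.
; The trail drops out of the way and is destroyed after a delay.
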(event `self.ReceiveBeginPlay`
  (`self.SetLifeSpan` 10.0)
  (`PrimitiveComponent.IgnoreActorWhenMoving` (`self.Sphere`) (`self.GetOwner`) true)
  (`ParticleSystemComponent.SetTemplate` (`self.Trail`) (`self.ProjectileTrail`)))

(event `self.ReceiveHit`
  (params (MyComp :type "PrimitiveComponent Object Reference") (Other :type "Actor Object Reference") (OtherComp :type "PrimitiveComponent Object Reference") (bSelfMoved :type Boolean) (HitLocation :type "Vector Structure") (HitNormal :type "Vector Structure") (NormalImpulse :type "Vector Structure") (Hit :type "HitResult Structure (by ref)"))
  (bind _trail (`self.Trail`))
  (bind (_returnvalue_roll _returnvalue_pitch _returnvalue_yaw) (`KismetMathLibrary.BreakRotator` (`KismetMathLibrary.Conv_VectorToRotator` (`self.HitNormal`))))
  (bind (_returnvalue_roll_2 _returnvalue_pitch_2 _returnvalue_yaw_2) (`KismetMathLibrary.BreakRotator` (`KismetMathLibrary.Conv_VectorToRotator` (`self.ImpactNormal`))))
  (bind (_returnvalue_x _returnvalue_y _returnvalue_z) (`KismetMathLibrary.BreakVector` (`SceneComponent.K2_GetComponentLocation` _trail)))
  (bind _returnvalue (`KismetMathLibrary.MakeRotator` _returnvalue_roll_2 (+ _returnvalue_pitch_2 -90.0) _returnvalue_yaw_2))
  (set `self.HitLocation` HitLocation)
  (set `self.HitNormal` HitNormal)
  (set `self.ImpactPoint` Hit_ImpactPoint)
  (set `self.ImpactNormal` Hit_ImpactNormal)
  (set `self.HitActor` Hit_HitActor)
  (set `self.HitComponent` Hit_HitComponent)
  (if (not (== (`self.HitActor`) (`self.GetOwner`)))
    (bind _outhit (`KismetSystemLibrary.SphereTraceSingle` :`Start` (`self.ImpactPoint`) :`End` (* (`self.ImpactPoint`) 0.99) :`Radius` 32.0 :`TraceChannel` "TraceTypeQuery1" :`bIgnoreSelf` false))
    (set `self.HitPhysMat` (`.PhysMat` (`GameplayStatics.BreakHitResult` _outhit)))
    (if (`KismetSystemLibrary.IsServer`)
      (`GameplayStatics.ApplyDamage` (`self.HitActor`) (`KismetMathLibrary.Conv_IntToDouble` (`self.Damage`)) null (`self.GetOwner`))
      (`AudioComponent.Stop` (`self.Audio`))
      ;[0 0 0] Impact momentum
      (`PrimitiveComponent.AddRadialImpulse` (`self.HitComponent`) (`self.HitLocation`) (`self.ImpulseRadius`) (`self.ImpulseStrength`) "RIF_Constant" true))
    (`|ExecutionSequence`
      (:`then_0`
        (`ActorComponent.K2_DestroyComponent` (`self.Sphere1`))
        (if (not (select `EPhysicalSurface` (`PhysicalMaterial.SurfaceType` (`self.HitPhysMat`)) :`SurfaceType2` true))
          (`GameplayStatics.SpawnDecalAtLocation` (`self.ImpactDecal`) (`self.DecalSize`) (`self.HitLocation`) (`KismetMathLibrary.MakeRotator` _returnvalue_roll (+ _returnvalue_pitch -180.0) (`KismetMathLibrary.RandomFloatInRange` _returnvalue_yaw 359.0)) (`self.DecalDuration`)))
        (`/Engine/EditorBlueprintResources/StandardMacros.IsValid` (`self.HitPhysMat`)
          (:`Is Valid`
            (switch `EPhysicalSurface` (`PhysicalMaterial.SurfaceType` (`self.HitPhysMat`))
              (:`SurfaceType_Default`
                (`self.HitEffect` (`self.ImpactEffect`) (`self.ImpactSound`) (`self.HitLocation`) :!label _label))
              (:`SurfaceType1`
                (`self.HitEffect` (select `/Game/YI_TankCollection/Blueprint/Master/Data/E_ProjectileType` (`self.Type`) :`NewEnumerator0` "/Game/YI_TankCollection/Particles/Master/P_Impact_Large.P_Impact_Large" :`NewEnumerator1` "/Game/YI_TankCollection/Particles/Master/P_Impact_Small.P_Impact_Small" :!type "ParticleSystem Object Reference") (`self.ImpactSound`) (`self.HitLocation`) _returnvalue))
              (:`SurfaceType2`
                (`self.HitEffect` (select `/Game/YI_TankCollection/Blueprint/Master/Data/E_ProjectileType` (`self.Type`) :`NewEnumerator0` "/Game/YI_TankCollection/Particles/Master/P_Explosion_Bomb.P_Explosion_Bomb" :`NewEnumerator1` "/Game/YI_TankCollection/Particles/Master/P_Impact_Metal.P_Impact_Metal" :!type "ParticleSystem Object Reference") (`self.ImpactSound`) (`self.HitLocation`) _returnvalue)
                ;[0 1 1] New
                (bind _asbp_tank_controller_chaos (cast `/Game/YI_TankCollection/Blueprint/Master/Controller/BP_TankController_Chaos` (`self.GetOwner`)))
                (`/Game/YI_TankCollection/Blueprint/Master/Controller/BP_TankController_Chaos.EventUpdateDamageUI` _asbp_tank_controller_chaos (`self.Damage`)))))
          (:`Is Not Valid`
            (goto _label))))
      (:`then_1`
        (`SceneComponent.K2_SetWorldLocation` _trail (`KismetMathLibrary.MakeVector` _returnvalue_x _returnvalue_y (- _returnvalue_z 500.0)) false false)
        (`KismetSystemLibrary.Delay` 10.0)
        (`ActorComponent.K2_DestroyComponent` (`self.Trail`))))))

(fn `UserConstructionScript`
  (set `ProjectileMovementComponent.InitialSpeed` (`self.InitialSpeed`) (`self.ProjectileMovement`))
  (set `ProjectileMovementComponent.ProjectileGravityScale` (`self.ProjectileGravityScale`) (`self.ProjectileMovement`)))