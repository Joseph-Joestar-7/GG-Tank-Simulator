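; Tank weapon component for BP_TankController_Chaos, handling up to five weapons with separate ammo, timed reloads and switching.
; Firing checks ammo, relays projectile spawn and effects through server-to-multicast events, then auto-reloads on empty, with looping timers for full-auto.
; Projectiles scatter in a cone from the vehicle's scattering values, and shots add radial and gun-bone recoil impulses.
; Tick traces from the current muzzle bone to update the crosshair aim point.
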(event `self.ReceiveBeginPlay`
  (bind _weapons (`self.Weapons`))
  ;[0 0 0] Begin Play ( Set Starting Weapon and ammo informations of all weaponery
  (bind _asbp_tank_controller_chaos (cast `/Game/YI_TankCollection/Blueprint/Master/Controller/BP_TankController_Chaos` (`self.GetOwner`)))
  (bind _output_get (set `self.Vehicle` _asbp_tank_controller_chaos))
  (set `self.VehicleMesh` (`Actor.GetComponentByClass` _output_get "/Script/Engine.SkeletalMeshComponent"))
  (for (_array_element _array_index) _weapons
    (switch `int` _array_index
      (:`0`
        (bind ((`WeaponAmmo_37_53EAF0244DFF34EBF2702FB18C2A7503` _weaponammo) (`ReloadTime_40_417535CD4D103BBEA4FDDFB27BECBC38` _reloadtime)) (break `/Game/YI_TankCollection/Blueprint/Master/Data/S_Weapon` _array_element))
        (bind _output_get_2 (set `self.Weapon1BaseAmmo` _weaponammo))
        (set `self.Weapon1CurrentAmmo` _output_get_2)
        (set `self.Weapon1ReloadTime` _reloadtime))
      (:`1`
        (bind _output_get_3 (set `self.Weapon2BaseAmmo` _weaponammo))
        (set `self.Weapon2CurrentAmmo` _output_get_3)
        (set `self.Weapon2ReloadTime` _reloadtime))
      (:`2`
        (bind _output_get_4 (set `self.Weapon3BaseAmmo` _weaponammo))
        (set `self.Weapon3CurrentAmmo` _output_get_4)
        (set `self.Weapon3ReloadTime` _reloadtime))
      (:`3`
        (bind _output_get_5 (set `self.Weapon4BaseAmmo` _weaponammo))
        (set `self.Weapon4CurrentAmmo` _output_get_5)
        (set `self.Weapon4ReloadTime` _reloadtime))
      (:`4`
        (bind _output_get_6 (set `self.Weapon5BaseAmmo` _weaponammo))
        (set `self.Weapon5CurrentAmmo` _output_get_6)
        (set `self.Weapon5ReloadTime` _reloadtime))))
  (set `self.CurrentWeapon` (`|GetArrayItem` _weapons))
  (set `self.Current WeaponIndex` 0))

(event `SERVER_FireEffect`
  (params (Particle :type "ParticleSystem Object Reference") (Sound :type "SoundBase Object Reference") (Location :type "Vector Structure") (Normal :type "Rotator Structure"))
  ;[0 0 0] Weapon Fire Effects
  (`self.MC_FireEffect` Particle Sound Location Normal))

(event `SERVER_SpawnProjectile`
  (params (Projectile :type "/Game/YI_TankCollection/Blueprint/Master/Projectiles/BP_ProjectileMaster Class Reference") (ProjectileSocket :type Name) (Damage :type Integer))
  ;[0 0 0] Weapon Projectile
  (`/Engine/EditorBlueprintResources/StandardMacros.IsValid` (`self.VehicleMesh`)
    (:`Is Valid`
      (`self.MC_SpawnProjectile` Projectile ProjectileSocket))))

(event `MC_FireEffect`
  (params (Particle :type "ParticleSystem Object Reference") (Sound :type "SoundBase Object Reference") (Location :type "Vector Structure") (Normal :type "Rotator Structure"))
  ;[0 0 0] Weapon Fire Effects
  (`GameplayStatics.SpawnEmitterAtLocation` Particle Location Normal)
  (`GameplayStatics.SpawnSoundAtLocation` Sound Location (struct) 1.0 1.0 0.0 null null))

(event `MC_SpawnProjectile`
  (params (Projectile :type "/Game/YI_TankCollection/Blueprint/Master/Projectiles/BP_ProjectileMaster Class Reference") (ProjectileSocket :type Name))
  (bind _vehiclemesh (`self.VehicleMesh`))
  (bind ((`ProjectileImpactEffect_45_93CB008844E3886F181A478474CCFCFB` _projectileimpacteffect) (`ProjectileImpactSound_46_21ED687949DC808843394988E5995731` _projectileimpactsound)) (break `/Game/YI_TankCollection/Blueprint/Master/Data/S_Weapon` (`self.CurrentWeapon`)))
  (bind (_returnvalue_location _returnvalue_rotation) (`KismetMathLibrary.BreakTransform` (`SceneComponent.GetSocketTransform` _vehiclemesh ProjectileSocket "RTS_World")))
  ;[0 0 0] Weapon Projectile
  (`self.IsLocallyControlled`
    (:`true`
      _)
    (:`false`
      _))
  (`/Engine/EditorBlueprintResources/StandardMacros.IsValid` _vehiclemesh
    (:`Is Valid`
      (bind _returnvalue (`|SpawnActorFromClass` Projectile (`KismetMathLibrary.MakeTransform` _returnvalue_location (`KismetMathLibrary.Conv_VectorToRotator` (`KismetMathLibrary.RandomUnitVectorInConeInDegrees` (`KismetMathLibrary.Conv_RotatorToVector` _returnvalue_rotation) (`KismetMathLibrary.DegAtan` (/ (`|GetArrayItem` (`/Game/YI_TankCollection/Blueprint/Master/Controller/BP_TankController_Chaos.FinalScattering` (`self.Vehicle`)) (`self.Current WeaponIndex`)) 100.0))))) "Undefined" "SelectDefaultAtRuntime" (`self.GetOwner`) 100 _projectileimpacteffect null _projectileimpactsound (`self.Vehicle`)))
      (add `/Game/YI_TankCollection/Blueprint/Master/Projectiles/BP_ProjectileMaster.HitEffect` _returnvalue (delegate `HitEffect_Event_0`)))))

(event `HitEffect_Event_0`
  (params (VFX :type "ParticleSystem Object Reference") (SFX :type "SoundBase Object Reference") (Location :type "Vector Structure") (Normal :type "Rotator Structure"))
  ;[0 0 0] Weapon Projectile
  (`self.SERVER_FireEffect` VFX SFX Location Normal))

(event `self.ReceiveTick`
  (params (DeltaSeconds :type "Float (single-precision)"))
  ;[0 0 0] Event Tick
  (`self.CrosshairTrace`))

(event `ReloadWeapon`
  (params (Weapon :type Integer))
  ;[0 0 0] Reload Weapon
  (`/Game/YI_TankCollection/Blueprint/Master/Controller/BP_TankController_Chaos.WeaponReloadUI` (`self.Vehicle`))
  (switch `int` Weapon
    (:`0`
      (if (and (!= (`self.Weapon1BaseAmmo`) (`self.Weapon1CurrentAmmo`)) (not (`self.ReloadingWeapon1`)))
        (set `self.ReloadingWeapon1` true)
        (`KismetSystemLibrary.Delay` (`self.Weapon1ReloadTime`))
        (set `self.Weapon1CurrentAmmo` (`self.Weapon1BaseAmmo`))
        (set `self.ReloadingWeapon1` false)))
    (:`1`
      (if (and (!= (`self.Weapon2BaseAmmo`) (`self.Weapon2CurrentAmmo`)) (not (`self.ReloadingWeapon2`)))
        (set `self.ReloadingWeapon2` true)
        (`KismetSystemLibrary.Delay` (`self.Weapon2ReloadTime`))
        (set `self.Weapon2CurrentAmmo` (`self.Weapon2BaseAmmo`))
        (set `self.ReloadingWeapon2` false)))
    (:`2`
      (if (and (!= (`self.Weapon3BaseAmmo`) (`self.Weapon3CurrentAmmo`)) (not (`self.ReloadingWeapon3`)))
        (set `self.ReloadingWeapon3` true)
        (`KismetSystemLibrary.Delay` (`self.Weapon3ReloadTime`))
        (set `self.Weapon3CurrentAmmo` (`self.Weapon3BaseAmmo`))
        (set `self.ReloadingWeapon3` false)))
    (:`3`
      (if (and (!= (`self.Weapon4BaseAmmo`) (`self.Weapon4CurrentAmmo`)) (not (`self.ReloadingWeapon4`)))
        (set `self.ReloadingWeapon4` true)
        (`KismetSystemLibrary.Delay` (`self.Weapon4ReloadTime`))
        (set `self.Weapon4CurrentAmmo` (`self.Weapon4BaseAmmo`))
        (set `self.ReloadingWeapon4` false)))
    (:`4`
      (if (and (!= (`self.Weapon5BaseAmmo`) (`self.Weapon5CurrentAmmo`)) (not (`self.ReloadingWeapon5`)))
        (set `self.ReloadingWeapon5` true)
        (`KismetSystemLibrary.Delay` (`self.Weapon5ReloadTime`))
        (set `self.Weapon5CurrentAmmo` (`self.Weapon5BaseAmmo`))
        (set `self.ReloadingWeapon5` false)))))

(event `SERVER_ChangeWeapon`
  (params (WeaponIndex :type Integer))
  ;[0 0 0] Change Weapon
  (`self.MC_ChangeWeapon` WeaponIndex))

(event `MC_ChangeWeapon`
  (params (WeaponIndex :type Integer))
  ;[0 0 0] Change Weapon
  (`self.ChangeWeapon` WeaponIndex))

(fn `ChangeWeapon`
  (params (WeaponIndex :type Integer))
  (if (`KismetArrayLibrary.Array_IsValidIndex` (`self.Weapons`) WeaponIndex)
    (set `self.CurrentWeapon` (`|GetArrayItem` (`self.Weapons`) WeaponIndex))
    (set `self.Current WeaponIndex` WeaponIndex)
    (`self.StopShooting`)))

(fn `CrosshairTrace`
  (bind _returnvalue (`SkinnedMeshComponent.GetSocketBoneName` (`self.VehicleMesh`) (`.ProjectileSocket_21_092B4E5841609FC59C74CAA6CFEA7D97` (break `/Game/YI_TankCollection/Blueprint/Master/Data/S_Weapon` (`self.CurrentWeapon`)))))
  (bind _returnvalue_2 (`SceneComponent.GetSocketLocation` (`self.VehicleMesh`) _returnvalue))
  (bind _outhit (`KismetSystemLibrary.LineTraceSingle` _returnvalue_2 (- (+ _returnvalue_2 (* (`KismetMathLibrary.GetForwardVector` (`SceneComponent.GetSocketRotation` (`self.VehicleMesh`) _returnvalue)) (`KismetMathLibrary.Clamp` 250000 0 (`KismetMathLibrary.FTrunc` (`/Game/YI_TankCollection/Blueprint/Master/Controller/BP_TankController_Chaos.CrosshairTraceClamp` (`self.Vehicle`)))))) (`KismetMathLibrary.MakeVector` 0.0 0.0 (`/Game/YI_TankCollection/Blueprint/Master/Controller/BP_TankController_Chaos.AimPointCorrectionUI` (`self.Vehicle`)))) "TraceTypeQuery2" false (`|MakeArray` (`self.GetOwner`))))
  (bind (_bblockinghit _binitialoverlap _time _distance _location _impactpoint _normal _impactnormal _physmat _hitactor _hitcomponent _hitbonename _bonename _hititem _elementindex _faceindex _tracestart _traceend) (`GameplayStatics.BreakHitResult` _outhit))
  (if _bblockinghit
    (set `self.TraceEnd` _impactpoint)
    (else
      (set `self.TraceEnd` _traceend))))

(fn `FireWeapon`
  (locals (GunSocketName :type Name))
  (bind (_weaponname _projectile _projectilesocket _projectiledamage _weaponammo _fullauto _firerate _reloadtime _fireeffect _fireeffectsocket _firesound) (break `/Game/YI_TankCollection/Blueprint/Master/Data/S_Weapon` (`self.CurrentWeapon`)))
  (bind (_output_weaponname _output_projectile _output_projectilesocket _output_projectiledamage _output_weaponammo _output_fullauto _output_firerate _output_reloadtime _output_fireeffect _output_fireeffectsocket _output_firesound _output_projectileimpacteffect _output_projectileimpactsound _output_turretrotationspeed _output_gunrotationspeed _output_horizontalrange _output_verticalrange _output_minscattering _output_aimingtime _output_scatteringstabangular _output_scatteringstablinear _output_impulse) (break `/Game/YI_TankCollection/Blueprint/Master/Data/S_Weapon` (`|GetArrayItem` (`self.Weapons`) (`self.Current WeaponIndex`))))
  (`self.CheckWeaponAmmo`)
  (`self.SERVER_SpawnProjectile` _projectile _projectilesocket _projectiledamage)
  (`self.SERVER_FireEffect` _fireeffect _firesound (`SceneComponent.GetSocketLocation` (`self.VehicleMesh`) _fireeffectsocket))
  (`self.UpdateWeaponAmmo`)
  ;[0 0 0] Weapon impulse
  ;;[0 1 1] New
  (set `local.GunSocketName` _output_projectilesocket)
  (`PrimitiveComponent.AddRadialImpulse` (`self.VehicleMesh`) (`SceneComponent.GetSocketLocation` (`self.VehicleMesh`) (`local.GunSocketName`)) 800.0 (/ _output_impulse 5.0) "RIF_Linear" false) ; For all rigid bodies
  (`PrimitiveComponent.AddImpulseAtLocation` (`self.VehicleMesh`) (* (* (`KismetMathLibrary.Conv_RotatorToVector` (`SceneComponent.GetSocketRotation` (`self.VehicleMesh`) (`local.GunSocketName`))) (-1.0 -1.0 -1.0)) _output_impulse) (`SceneComponent.GetSocketLocation` (`self.VehicleMesh`) (`local.GunSocketName`)) "main_gun") ; For 1 rigid body
  (`self.WeaponFire` (`self.Current WeaponIndex`)))

(fn `StartShooting`
  (bind (_weaponname _projectile _projectilesocket _projectiledamage _weaponammo _fullauto _firerate) (break `/Game/YI_TankCollection/Blueprint/Master/Data/S_Weapon` (`self.CurrentWeapon`)))
  (`self.FireWeapon`)
  (if _fullauto
    (bind _returnvalue (`KismetSystemLibrary.K2_SetTimer` null "FireWeapon" _firerate true))
    (set `self.FullAuto` _returnvalue)))

(fn `StopShooting`
  (`KismetSystemLibrary.K2_ClearAndInvalidateTimerHandle` (`self.FullAuto`)))

(fn `UpdateWeaponAmmo`
  (switch `int` (`self.Current WeaponIndex`)
    (:`0`
      (set `self.Weapon1CurrentAmmo` (- (`self.Weapon1CurrentAmmo`) 1))
      (if (== (`self.Weapon1CurrentAmmo`) 0)
        (`self.ReloadWeapon` 0)))
    (:`1`
      (set `self.Weapon2CurrentAmmo` (- (`self.Weapon2CurrentAmmo`) 1))
      (if (== (`self.Weapon2CurrentAmmo`) 0)
        (`self.ReloadWeapon` 1)))
    (:`2`
      (set `self.Weapon3CurrentAmmo` (- (`self.Weapon3CurrentAmmo`) 1))
      (if (== (`self.Weapon3CurrentAmmo`) 0)
        (`self.ReloadWeapon` 2)))
    (:`3`
      (set `self.Weapon4CurrentAmmo` (- (`self.Weapon4CurrentAmmo`) 1))
      (if (== (`self.Weapon4CurrentAmmo`) 0)
        (`self.ReloadWeapon` 3)))
    (:`4`
      (set `self.Weapon5CurrentAmmo` (- (`self.Weapon5CurrentAmmo`) 1))
      (if (== (`self.Weapon5CurrentAmmo`) 0)
        (`self.ReloadWeapon` 4)))))