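; BrokenCar is a damageable wrecked-car prop for the DesertTown environment.
; The construction script picks one of two meshes and creates a dynamic material instance for tint, sand dust and light glow.
; A lights toggle and strength value drive both that glow and the headlight and brake light intensities.
; Damage drains a health component, whose death event activates fire and explosion effects and darkens the tint to a scorched brown.
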(event `self.ReceiveAnyDamage`
  (params (Damage :type "Float (single-precision)") (DamageType :type "DamageType Object Reference") (InstigatedBy :type "Controller Object Reference") (DamageCauser :type "Actor Object Reference"))
  (`/Game/Components/BPC_Health.ChangeValue` (`self.BPC_Health`) (* Damage -1.0)))

(event `self.BPC_Health.HasDied`
  (`ActorComponent.Activate` (`self.P_Fire_Big`) true)
  (`ActorComponent.Activate` (`self.P_Explosion_Big_A`) true)
  (bind _output_get (set `self.Tint` (struct :`R` 0.089583 :`G` 0.050476 :`A` 1.0)))
  (`MaterialInstanceDynamic.SetVectorParameterValue` (`self.DMI_Headlight`) "Tint" _output_get))

(fn `UserConstructionScript`
  (bind _staticmesh (`self.StaticMesh`))
  (bind _dmi_headlight (`self.DMI_Headlight`))
  (bind _lights_strength (`self.Lights_Strength`))
  (bind _dmi_headlight_2 (`self.DMI_Headlight`))
  (if (`self.SwapDamage`)
    (`StaticMeshComponent.SetStaticMesh` _staticmesh "/Game/DesertTown/Models/BrokenCar.BrokenCar")
    (else
      (`StaticMeshComponent.SetStaticMesh` _staticmesh "/Game/DesertTown/Models/BrokenCar_B.BrokenCar_B")))
  (bind _returnvalue (`PrimitiveComponent.CreateDynamicMaterialInstance` (`self.StaticMesh`) 0 "/Game/DesertTown/Materials/BrokenCar.BrokenCar" "None"))
  (set `self.DMI_Headlight` _returnvalue)
  (`MaterialInstanceDynamic.SetVectorParameterValue` _dmi_headlight_2 "Tint" (`self.Tint`))
  (`MaterialInstanceDynamic.SetScalarParameterValue` _dmi_headlight_2 "SandOpacity" (`self.Top Dust`))
  (if (`self.Lights_Toggle`)
    (`MaterialInstanceDynamic.SetScalarParameterValue` _dmi_headlight "Lights" _lights_strength)
    (`LightComponent.SetIntensity` (`self.Headlight_L`) (* _lights_strength 10000.0))
    (`LightComponent.SetIntensity` (`self.Headlight_R`) (* _lights_strength 10000.0))
    (`LightComponent.SetIntensity` (`self.Brakelight_L`) (* _lights_strength 100.0))
    (`LightComponent.SetIntensity` (`self.Brakelight_R`) (* _lights_strength 100.0))
    (else
      (`MaterialInstanceDynamic.SetScalarParameterValue` _dmi_headlight "Lights" 0.0)
      (`LightComponent.SetIntensity` (`self.Headlight_R`) 0.0)
      (`LightComponent.SetIntensity` (`self.Headlight_L`) 0.0)
      (`LightComponent.SetIntensity` (`self.Brakelight_R`) 0.0)
      (`LightComponent.SetIntensity` (`self.Brakelight_L`) 0.0))))