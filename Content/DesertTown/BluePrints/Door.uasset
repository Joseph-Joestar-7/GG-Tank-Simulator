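; Interactive door for the DesertTown area that the player opens and closes with the E key.
; Overlapping its sphere enables input for player controller 0, and nothing in the graph disables it afterwards.
; Each press flips the OpenClose flag, plays the audio and runs the DoorAnim timeline from start or in reverse, setting the mesh's relative yaw.
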(event `self.ReceiveBeginPlay`)

(event `self.ReceiveActorBeginOverlap`
  (params (OtherActor :type "Actor Object Reference")))

(event `self.Sphere.OnComponentBeginOverlap`
  (params (OtherActor :type "Actor Object Reference") (OtherComp :type "PrimitiveComponent Object Reference") (OtherBodyIndex :type Integer) (bFromSweep :type Boolean) (SweepResult :type "HitResult Structure (by ref)"))
  (`self.EnableInput` (`GameplayStatics.GetPlayerController` 0)))

(event `self.ReceiveTick`
  (params (DeltaSeconds :type "Float (single-precision)")))

(event `Key|E`
  (params (Key :type "Key Structure" :default "AnyKey"))
  (bind _audio (`self.Audio`))
  (:`Pressed`
    (if (`self.Open_Close`)
      (set `self.Open_Close` false)
      (`AudioComponent.Play` _audio 0.0)
      (bind (_direction _dooranim) (`Timeline|DoorAnim` :!via `PlayFromStart` :!label _label)
        (:`Update`
          (`SceneComponent.K2_SetRelativeRotation` (`self.StaticMesh`) (`KismetMathLibrary.MakeRotator` 0.0 0.0 _dooranim) false false)))
      (else
        (set `self.Open_Close` true)
        (`AudioComponent.Play` _audio 0.0)
        (goto _label :!via `Reverse`)))))

(fn `UserConstructionScript`)