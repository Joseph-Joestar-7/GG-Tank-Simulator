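; Radio tower actor for the desert town with a blinking red warning light.
; The construction script creates a dynamic instance of the red light material on the tower mesh.
; From BeginPlay, an endless delay loop switches that material's emissive strength and a point light's intensity off and on together at one-second intervals.
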(event `self.ReceiveBeginPlay`
  (bind _dmi (`self.DMI`))
  (bind _pointlight (`self.PointLight`))
  (`KismetSystemLibrary.Delay` 1.0 :!label _label)
  (`MaterialInstanceDynamic.SetScalarParameterValue` _dmi "EmissiveStrength" 0.0)
  (`LightComponent.SetIntensity` _pointlight 0.0)
  (`KismetSystemLibrary.Delay` 1.0)
  (`MaterialInstanceDynamic.SetScalarParameterValue` _dmi "EmissiveStrength" 200.0)
  (`LightComponent.SetIntensity` _pointlight 15000.0)
  (goto _label))

(event `self.ReceiveActorBeginOverlap`
  (params (OtherActor :type "Actor Object Reference")))

(event `self.ReceiveTick`
  (params (DeltaSeconds :type "Float (single-precision)")))

(fn `UserConstructionScript`
  (bind _returnvalue (`PrimitiveComponent.CreateDynamicMaterialInstance` (`self.StaticMesh`) 1 "/Game/DesertTown/Materials/RedLight.RedLight"))
  (set `self.DMI` _returnvalue))