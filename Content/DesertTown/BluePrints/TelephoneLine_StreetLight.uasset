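; Desert town street light prop with telephone line spline meshes, configured entirely in the construction script with no runtime logic.
; Two spline meshes share a curve between start and offset end transforms, their tangents pitched by a hang amount and scaled by span length to shape the sag.
; The light mesh takes a set angle and height, while a toggle and intensity drive both its dynamic material and spotlight.
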(event `self.ReceiveBeginPlay`)

(event `self.ReceiveActorBeginOverlap`
  (params (OtherActor :type "Actor Object Reference")))

(event `self.ReceiveTick`
  (params (DeltaSeconds :type "Float (single-precision)")))

(fn `UserConstructionScript`
  (bind _dmi (`self.DMI`))
  (bind _lightintensity (`self.LightIntensity`))
  (bind _spotlight (`self.SpotLight`))
  (bind _streetlight (`self.StreetLight`))
  (bind _hangamount (`self.HangAmount`))
  (bind _location (.location (`self.Start transform`)))
  (bind _returnvalue (+ (.location (`self.End Transform`)) (`self.Distance`)))
  (bind _returnvalue_2 (`KismetMathLibrary.VSize` (- _location _returnvalue)))
  (`SplineMeshComponent.SetStartAndEnd` (`self.SplineMesh`) _location (* (* (`KismetMathLibrary.GetForwardVector` (`KismetMathLibrary.ComposeRotators` (.rotation (`self.Start transform`)) (* _hangamount -1.0))) (.scale (`self.Start transform`))) _returnvalue_2) _returnvalue (* (* (`KismetMathLibrary.GetForwardVector` (`KismetMathLibrary.ComposeRotators` (.rotation (`self.End Transform`)) _hangamount)) (.scale (`self.End Transform`))) _returnvalue_2))
  (`SplineMeshComponent.SetStartAndEnd` (`self.SplineMesh1`) _location (* (* (`KismetMathLibrary.GetForwardVector` (`KismetMathLibrary.ComposeRotators` (.rotation (`self.Start transform`)) (* _hangamount -1.0))) (.scale (`self.Start transform`))) _returnvalue_2) _returnvalue (* (* (`KismetMathLibrary.GetForwardVector` (`KismetMathLibrary.ComposeRotators` (.rotation (`self.End Transform`)) _hangamount)) (.scale (`self.End Transform`))) _returnvalue_2))
  (`SceneComponent.K2_SetRelativeRotation` _streetlight (`KismetMathLibrary.MakeRotator` 0.0 0.0 (`self.LightAngle`)) false false)
  (`SceneComponent.K2_AddWorldOffset` _streetlight (`KismetMathLibrary.MakeVector` 0.0 0.0 (`self.LightHeight`)) false false)
  (bind _returnvalue_3 (`PrimitiveComponent.CreateDynamicMaterialInstance` (`self.StreetLight`) 0 "/Game/DesertTown/Materials/StreetLight.StreetLight"))
  (set `self.DMI` _returnvalue_3)
  (if (`self.Light_Toggle`)
    (`MaterialInstanceDynamic.SetScalarParameterValue` _dmi "LightIntensity" _lightintensity)
    (`LightComponent.SetIntensity` _spotlight (* _lightintensity 1000.0))
    (else
      (`MaterialInstanceDynamic.SetScalarParameterValue` _dmi "LightIntensity" 0.0)
      (`LightComponent.SetIntensity` _spotlight 0.0))))