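; Telephone line actor that stretches a sagging wire between a start and end transform for the DesertTown environment.
; The construction script sets the same start, end and tangents on two spline mesh components, with a Distance offset added to the end position.
; Tangent directions come from each transform's rotation combined with an opposing HangAmount, then are multiplied by its scale and the span length to shape the sag.
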(event `self.ReceiveBeginPlay`)

(event `self.ReceiveActorBeginOverlap`
  (params (OtherActor :type "Actor Object Reference")))

(event `self.ReceiveTick`
  (params (DeltaSeconds :type "Float (single-precision)")))

(fn `UserConstructionScript`
  (bind _hangamount (`self.HangAmount`))
  (bind _location (.location (`self.Start transform`)))
  (bind _returnvalue (+ (.location (`self.End Transform`)) (`self.Distance`)))
  (bind _returnvalue_2 (`KismetMathLibrary.VSize` (- _location _returnvalue)))
  (`SplineMeshComponent.SetStartAndEnd` (`self.SplineMesh`) _location (* (* (`KismetMathLibrary.GetForwardVector` (`KismetMathLibrary.ComposeRotators` (.rotation (`self.Start transform`)) (* _hangamount -1.0))) (.scale (`self.Start transform`))) _returnvalue_2) _returnvalue (* (* (`KismetMathLibrary.GetForwardVector` (`KismetMathLibrary.ComposeRotators` (.rotation (`self.End Transform`)) _hangamount)) (.scale (`self.End Transform`))) _returnvalue_2))
  (`SplineMeshComponent.SetStartAndEnd` (`self.SplineMesh1`) _location (* (* (`KismetMathLibrary.GetForwardVector` (`KismetMathLibrary.ComposeRotators` (.rotation (`self.Start transform`)) (* _hangamount -1.0))) (.scale (`self.Start transform`))) _returnvalue_2) _returnvalue (* (* (`KismetMathLibrary.GetForwardVector` (`KismetMathLibrary.ComposeRotators` (.rotation (`self.End Transform`)) _hangamount)) (.scale (`self.End Transform`))) _returnvalue_2)))